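; Debris_Master is a debris actor whose Lights component shows its reward type: None, Energy, KCell or Artefact.
; Construction runs Init, which applies the reward's transparent material to alternating Lights material slots and randomises the scale of StaticMesh and Lights on each axis.
; At BeginPlay it caches the first KaijuPlayer_BP and starts a one-second looping timer that sets Lights visibility from the player's SimulationFinished flag.
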(event Custom|ChekcSimFInished
  (Rendering|SetVisibility (Variables|Default|GetLights) (Variables|/Game/Blueprints/Actors/KaijuPlayer_BP.KaijuPlayer_BP_C|Get_simulationFinished (Variables|Default|GetPlayerRef)) false))

(event EventBeginPlay
  (|CallParentFunction)
  (bind _outactors (Actor|GetAllActorsOfClass "/Game/Blueprints/Actors/KaijuPlayer_BP.KaijuPlayer_BP_C"))
  (Variables|Default|SetPlayerRef (Utilities|Array|Get(acopy) _outactors))
  (Utilities|Time|SetTimerbyEvent (delegate Custom|ChekcSimFInished) 1.0 true))

(event Collision|EventActorBeginOverlap
  (params (OtherActor :type Actor%20Object%20Reference)))

(event EventTick
  (params (DeltaSeconds :type Float%20%28single-precision%29)))

(fn ConstructionScript
  (|CallParentFunction)
  (CallFunction|Init))

(fn Init
  (bind _returnvalue (Math|Random|RandomFloatinRange 0.65 1.0))
  (for _index (range 0 8)
    (switch int _index
      (:0
        _)
      (:2
        _)
      (:4
        _)
      (:6
        _))
    (Rendering|Material|SetMaterial (Variables|Default|GetLights) _index (Utilities|Select :Index (Variables|Default|GetRewardType) :NewEnumerator0 "/Game/Materials/Transparent_Material_2.Transparent_Material_2" :NewEnumerator1 "/Game/Materials/Transparent_Material_1.Transparent_Material_1" :NewEnumerator2 "/Game/Materials/Transparent_Material_3.Transparent_Material_3" :NewEnumerator3 "/Game/Materials/Transparent_Material_4.Transparent_Material_4")))
  (Transformation|SetRelativeScale3D (Variables|Default|GetStaticMesh) (Math|Vector|MakeVector _returnvalue _returnvalue _returnvalue)))