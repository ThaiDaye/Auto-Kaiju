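; Actor_Master is an actor Blueprint, apparently a master class for units, that holds health, defence and death state.
; On BeginPlay, InitiateUnit sets Health to HealthMax.
; CalculateDamage passes incoming damage and Defence through CalculateDefence, subtracts the result from Health clamped between zero and HealthMax, and flags IsDead when health runs out.
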(event EventBeginPlay
  (CallFunction|InitiateUnit))

(fn ConstructionScript)

(fn InitiateUnit
  (Variables|Default|SetHealth (Variables|Default|GetHealthMax)))

(fn CalculateDamage
  (params (Damage :type Float%20%28single-precision%29))
  (bind _output_get (Variables|Default|SetHealth (Math|Float|Clamp(Float) (- (Variables|Default|GetHealth) (Utilities|CalculateDefence Damage (Variables|Default|GetDefence))) 0.0 (Variables|Default|GetHealthMax))))
  (if (<= _output_get 0.0)
    (Variables|Default|SetIsDead true)))