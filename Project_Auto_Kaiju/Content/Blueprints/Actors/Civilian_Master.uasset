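; Civilian master actor representing a crowd as randomly scattered, scaled mesh instances, one per point of max health, built at construction and BeginPlay.
; Every five seconds a sphere trace looks for Kaiju, points an arrow roughly away from any found and opens a movement gate, closing it after a random delay.
; A fast looping timer sweeps the capsule along the arrow while the gate is open; hits redirect the arrow off the surface normal.
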(event Custom|Event_SpawnCivilians
  (bind _returnvalue (Math|Random|RandomFloatinRange 0.02 0.05))
  (bind _instancedstaticmesh (Variables|Default|GetInstancedStaticMesh))
  (bind _sphere (Variables|Default|GetSphere))
  (bind _groupradius (Variables|Default|GetGroupRadius))
  (bind _returnvalue_2 (Transformation|GetWorldLocation _sphere))
  ;[1 1 1] spawn civilians
  (Components|InstancedStaticMesh|ClearInstances _instancedstaticmesh)
  (Components|Sphere|SetSphereRadius _sphere (Variables|Default|GetGroupRadius) true)
  (for _index (range 1 (Math|Float|Round (Variables|Default|GetHealthMax)))
    (Class|InstancedStaticMeshComponent|AddInstanceWorldSpace _instancedstaticmesh (Math|Transform|MakeTransform (Math|Vector|Lerp(Vector) (Math|Random|RandomPointinBoundingBox _returnvalue_2 (Math|Vector|MakeVector _groupradius _groupradius 2.0)) _returnvalue_2 (Math|Random|RandomFloatinRange 0.0 1.0)) (Math|Rotator|MakeRotator 0.0 0.0 (Math|Random|RandomFloatinRange 0.0 1.8e+02)) (Math|Vector|MakeVector _returnvalue _returnvalue (Math|Random|RandomFloatinRange 0.05 0.1))))))

(event Custom|Event_RunAway
  ;[1 1 1] Run away
  (Utilities|FlowControl|Gate true
    (:Exit
      (Transformation|AddWorldOffset (Variables|Default|GetCapsuleComponent) (* (Math|Vector|GetForwardVector (Variables|Default|GetArrow1)) (Math|Random|RandomFloatinRange 0.2 0.4)) true false))))

(event Custom|Event_TurnAway
  (bind _capsulecomponent (Variables|Default|GetCapsuleComponent))
  (bind _returnvalue (Transformation|GetWorldLocation _capsulecomponent))
  ;[1 1 1] turn away
  (bind _outhits (Collision|MultiSphereTraceForObjects _returnvalue _returnvalue (* (Variables|Default|GetGroupRadius) 5.0) (Utilities|Array|MakeArray "ObjectTypeQuery3") false 0 "None"))
  (for _array_element _outhits
    (bind _askaiju_master (Utilities|Casting|CastToKaiju_Master (.HitActor (Collision|BreakHitResult _array_element))))
    (Transformation|SetWorldRotation (Variables|Default|GetArrow1) (Math|Rotator|MakeRotator (.roll (Transformation|GetActorRotation _askaiju_master)) (.pitch (Transformation|GetActorRotation _askaiju_master)) (+ (.yaw (Math|Rotator|FindLookatRotation (Transformation|GetActorLocation _askaiju_master) (Transformation|GetActorLocation))) (Math|Random|RandomFloatinRange -45.0 45.0))) false false)
    (CallFunction|EventTurnAwayEnd)))

(event Custom|Event_TurnAwayEnd
  ;[1 1 1] Run away
  (Utilities|FlowControl|Sequence
    (:then_0
      (Utilities|FlowControl|Gate true) ; enters at Open
    )
    (:then_1
      (Utilities|FlowControl|Delay (Math|Random|RandomFloatinRange 1e+01 2e+01))
      (Utilities|FlowControl|Gate true) ; enters at Close
    )))

(event EventBeginPlay
  ;[1 1 1] begin play
  (|CallParentFunction)
  (CallFunction|EventSpawnCivilians)
  (Utilities|Time|SetTimerbyEvent (delegate Custom|Event_RunAway) 0.01 true)
  (Utilities|Time|SetTimerbyEvent (delegate Custom|Event_TurnAway) 5.0 true))

(event Collision|EventHit
  (params (MyComp :type Primitive%20Component%20Object%20Reference) (Other :type Actor%20Object%20Reference) (OtherComp :type Primitive%20Component%20Object%20Reference) (bSelfMoved :type Boolean) (HitLocation :type Vector :default "0, 0, 0") (HitNormal :type Vector :default "0, 0, 0") (NormalImpulse :type Vector :default "0, 0, 0") (Hit :type Hit%20Result%20Structure%20%28by%20ref%29))
  (bind _returnvalue (Transformation|GetActorRotation))
  ;[1 1 1] on hit (turn)
  (Transformation|SetWorldRotation (Variables|Default|GetArrow1) (Math|Rotator|MakeRotator (.roll _returnvalue) (.pitch _returnvalue) (+ (.yaw (Math|Conversions|RotationFromXVector HitNormal)) (Math|Random|RandomFloatinRange -45.0 45.0))) false false))

(fn ConstructionScript
  (|CallParentFunction)
  (CallFunction|EventSpawnCivilians))