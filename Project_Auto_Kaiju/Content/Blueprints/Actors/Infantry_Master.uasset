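; Infantry squad actor that seeks out and attacks living Kaiju_Master actors, drawn as scattered instanced meshes whose count scales with HealthMax.
; A periodic sphere trace picks the target and steers DirectionArrow toward it, with random yaw spread widening up close, then opens a gate for timed bursts of swept movement.
; Separate timers aim and flash AutoArrow while dealing in-range damage scaled by HealthMax.
; Collisions redirect movement along the randomized hit normal.
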(event Custom|Event_SpawnCivilians
  (bind _returnvalue (Math|Random|RandomFloatinRange 0.02 0.05))
  (bind _instancedstaticmesh (Variables|Default|GetInstancedStaticMesh))
  (bind _sphere (Variables|Default|GetSphere))
  (bind _groupradius (Variables|Default|GetGroupRadius))
  (bind _returnvalue_2 (Transformation|GetWorldLocation _sphere))
  ;[1 1 1] spawn civilians
  (Components|InstancedStaticMesh|ClearInstances _instancedstaticmesh)
  (Components|Sphere|SetSphereRadius _sphere (Variables|Default|GetGroupRadius) true)
  (for _index (range 1 (Math|Float|Round (* (Variables|Default|GetHealthMax) 0.2)))
    (Class|InstancedStaticMeshComponent|AddInstanceWorldSpace _instancedstaticmesh (Math|Transform|MakeTransform (Math|Vector|Lerp(Vector) (Math|Random|RandomPointinBoundingBox _returnvalue_2 (Math|Vector|MakeVector _groupradius _groupradius 2.0)) _returnvalue_2 (Math|Random|RandomFloatinRange 0.25 1.0)) (Math|Rotator|MakeRotator 0.0 0.0 (Math|Random|RandomFloatinRange 0.0 1.8e+02)) (Math|Vector|MakeVector _returnvalue _returnvalue (Math|Random|RandomFloatinRange 0.05 0.1))))))

(event Custom|Aim
  (bind _target (Variables|Default|GetTarget))
  ;[1 1 1] aim
  (Utilities|IsValid _target
    (:Is%20Valid
      (Transformation|SetWorldRotation (Variables|Default|GetAutoArrow) (Math|Rotator|FindLookatRotation (Transformation|GetActorLocation) (Transformation|GetActorLocation _target)) false false))))

(event Custom|Event_RunTowards
  ;[1 1 1] Run towards
  (Utilities|FlowControl|Gate true
    (:Exit
      (Transformation|AddWorldOffset (Variables|Default|GetCapsuleComponent) (* (Math|Vector|GetForwardVector (Variables|Default|GetDirectionArrow)) (* (Variables|Default|GetMoveSpeed) 0.005)) true false))))

(event Custom|Event_TurnAway
  (bind _returnvalue (Transformation|GetActorLocation))
  (bind _capsulecomponent (Variables|Default|GetCapsuleComponent))
  (bind _returnvalue_2 (Transformation|GetWorldLocation _capsulecomponent))
  ;[1 1 1] turn towards
  (bind _outhits (Collision|MultiSphereTraceForObjects _returnvalue_2 _returnvalue_2 (* (Variables|Default|GetGroupRadius) 7.5) (Utilities|Array|MakeArray "ObjectTypeQuery3") false 0 "None"))
  (for _array_element _outhits
    (bind _askaiju_master (Utilities|Casting|CastToKaiju_Master (.HitActor (Collision|BreakHitResult _array_element))))
    (if (not (Variables|/Game/Blueprints/Actors/Masters/Actor_Master.Actor_Master_C|GetIsDead _askaiju_master))
      (Transformation|SetWorldRotation (Variables|Default|GetDirectionArrow) (Math|Rotator|MakeRotator (.roll (Transformation|GetActorRotation _askaiju_master)) (.pitch (Transformation|GetActorRotation _askaiju_master)) (+ (.yaw (Math|Rotator|FindLookatRotation _returnvalue (Transformation|GetActorLocation _askaiju_master))) (Math|Random|RandomFloatinRange (* (Math|Float|Lerp 9e+01 0.0 (Math|Float|Clamp(Float) (* (Math|Vector|VectorLength (- _returnvalue (Transformation|GetActorLocation _askaiju_master))) (* (Variables|Default|GetAttackRange) 5e-06)))) -1.0) (Math|Float|Lerp 9e+01 0.0 (Math|Float|Clamp(Float) (* (Math|Vector|VectorLength (- _returnvalue (Transformation|GetActorLocation _askaiju_master))) (* (Variables|Default|GetAttackRange) 5e-06))))))) false false)
      (Variables|Default|SetTarget _askaiju_master)
      (CallFunction|EventTurnTowardsEnd))))

(event Custom|Event_TurnTowardsEnd
  ;[1 1 1] Run towards
  (Utilities|FlowControl|Sequence
    (:then_0
      (Utilities|FlowControl|Gate true) ; enters at Open
    )
    (:then_1
      (Utilities|FlowControl|Delay (Math|Random|RandomFloatinRange 1e+01 3e+01))
      (Utilities|FlowControl|Gate true) ; enters at Close
    )))

(event Custom|AutoAttack
  (bind _target (Variables|Default|GetTarget))
  (bind _autoarrow (Variables|Default|GetAutoArrow))
  ;[1 1 1] autoattack
  (Utilities|IsValid _target
    (:Is%20Valid
      (if (<= (Transformation|GetDistanceTo _target) (Variables|Default|GetAttackRange))
        (Default|TakeDamage _target (* (Variables|Default|GetAttackDamage) (* (Variables|Default|GetHealthMax) 0.2)) self)
        (Rendering|SetVisibility _autoarrow true false)
        (Utilities|FlowControl|Delay 0.2)
        (Rendering|SetVisibility _autoarrow false false)))))

(event EventBeginPlay
  ;[1 1 1] begin play
  (|CallParentFunction)
  (CallFunction|EventSpawnCivilians)
  (Utilities|Time|SetTimerbyEvent (delegate Custom|Event_RunTowards) 0.01 true)
  (Utilities|Time|SetTimerbyEvent (delegate Custom|Event_TurnAway) 7.5 true)
  (Utilities|Time|SetTimerbyEvent (delegate Custom|Aim) 0.1 true)
  (Utilities|Time|SetTimerbyEvent (delegate Custom|AutoAttack) (Utilities|CalculateAttackSpeed (Variables|Default|GetAttackSpeed)) true))

(event Collision|EventHit
  (params (MyComp :type Primitive%20Component%20Object%20Reference) (Other :type Actor%20Object%20Reference) (OtherComp :type Primitive%20Component%20Object%20Reference) (bSelfMoved :type Boolean) (HitLocation :type Vector :default "0, 0, 0") (HitNormal :type Vector :default "0, 0, 0") (NormalImpulse :type Vector :default "0, 0, 0") (Hit :type Hit%20Result%20Structure%20%28by%20ref%29))
  (bind _returnvalue (Transformation|GetActorRotation))
  ;[1 1 1] on hit (turn)
  (Transformation|SetWorldRotation (Variables|Default|GetDirectionArrow) (Math|Rotator|MakeRotator (.roll _returnvalue) (.pitch _returnvalue) (+ (.yaw (Math|Conversions|RotationFromXVector HitNormal)) (Math|Random|RandomFloatinRange -45.0 45.0))) false false))

(fn ConstructionScript
  (|CallParentFunction)
  (CallFunction|EventSpawnCivilians))