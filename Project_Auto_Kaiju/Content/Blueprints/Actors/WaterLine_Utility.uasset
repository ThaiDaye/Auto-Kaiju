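; WaterLine_Utility is an actor that animates the position of its static mesh when play begins.
; BeginPlay starts a timeline whose track drives a Lerp, sliding the mesh a short distance along its relative X axis.
; The overlap and tick events are disabled placeholders, and the construction script only calls its parent.
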(event EventBeginPlay
  (|CallParentFunction)
  (bind _newtrack_0 (Timeline|Timeline_0 PlayFromStart)
    (:Update
      (Transformation|SetRelativeLocation (Variables|Default|GetStaticMesh) (Math|Vector|MakeVector (Math|Float|Lerp 0.0 2e+01 _newtrack_0) 0.0 0.0) false false))))

(event Collision|EventActorBeginOverlap
  (params (OtherActor :type Actor%20Object%20Reference))
  (|CallParentFunction OtherActor) ; This node is disabled and will not be called.\nDrag off pins to build functionality.
)

(event EventTick
  (params (DeltaSeconds :type Float%20%28single-precision%29))
  (|CallParentFunction DeltaSeconds) ; This node is disabled and will not be called.\nDrag off pins to build functionality.
)

(fn ConstructionScript
  (|CallParentFunction))