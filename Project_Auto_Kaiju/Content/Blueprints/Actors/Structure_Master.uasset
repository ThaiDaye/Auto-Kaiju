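; Structure_Master is a base destructible building that extends a parent unit class with height-based setup, civilian spawning and a collapse on death.
; Initiation picks the nav area and cube height from Height, randomizes the footprint, and disables cube collision at height zero.
; Each hit has a chance to spawn a Civilian_Master at a random entrance and trigger its turn-away event.
; Death disables collision, then a timeline jitters and sinks the cube before destroying the actor.
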(event EventBeginPlay
  ;[1 1 1] begin play
  (|CallParentFunction))

(event EventEventIsDead
  (bind _cube (Variables|Default|GetCube))
  ;[1 1 1] On Death
  (Utilities|FlowControl|DoOnce false
    (:Completed
      (Collision|SetCollisionResponsetoAllChannels _cube "ECR_Ignore")
      (Collision|SetCollisionEnabled _cube "NoCollision")
      (Components|DestroyComponent (Variables|Default|GetBox))
      (bind (_direction _newtrack_0 _newtrack_1 _newtrack_2) (Timeline|Timeline_0 PlayFromStart)
        (:Update
          (Transformation|SetRelativeLocation _cube (Math|Vector|MakeVector (Math|Float|Lerp -0.75 0.75 _newtrack_1) (Math|Float|Lerp -0.75 0.75 _newtrack_2) (Math|Float|Lerp -4e+01 -2.5e+02 _newtrack_0)) false false))
        (:Finished
          (Actor|DestroyActor))))))

(fn ConstructionScript
  (|CallParentFunction))

(fn InitiateUnit
  (bind _returnvalue (Math|Random|RandomFloatinRange 0.3 0.5))
  (bind _height (Variables|Default|GetHeight))
  (bind _cube (Variables|Default|GetCube))
  (|CallParentFunction)
  (Class|NavModifierComponent|SetAreaClass (Variables|Default|GetNavModifier) (Utilities|Select :Index _height :Option%200 0 :Option%201 "/Game/Blueprints/NavMesh/Height_One_Area.Height_One_Area_C" :Option%202 "/Game/Blueprints/NavMesh/Height_One_Area.Height_One_Area_C"))
  (Transformation|SetRelativeScale3D _cube (Math|Vector|MakeVector _returnvalue _returnvalue (Utilities|Select :Index _height :Option%200 0.15 :Option%201 0.5 :Option%202 0.8 :Option%203 1.25)))
  (if (== _height 0)
    (Collision|SetCollisionEnabled _cube "NoCollision")))

(fn TakeDamage
  (params (Damage :type Float%20%28single-precision%29) (Owner :type Actor%20Master%20Object%20Reference))
  (bind _isdead (|CallParentFunction Damage Owner))
  (CallFunction|SpawnCivilians)
  (return _isdead))

(fn SpawnCivilians
  (if (<= (Math|Random|RandomFloatinRange 0.0 1.0) (Math|Float|MakeLiteralFloat 0.25))
    (bind _returnvalue (Game|SpawnActorfromClass "/Game/Blueprints/Actors/Civilian_Master.Civilian_Master_C" (Math|Transform|MakeTransform (Transformation|GetWorldLocation (Utilities|Select :Index (Math|Random|RandomIntegerinRange 0 3) :Option%200 (Variables|Default|GetEntrance_1) :Option%201 (Variables|Default|GetEntrance_2) :Option%202 (Variables|Default|GetEntrance_3) :Option%203 (Variables|Default|GetEntrance_4))) (Math|Rotator|MakeRotator 0.0 0.0 (Math|Random|RandomFloatinRange 0.0 1.8e+02))) "AdjustIfPossibleButAlwaysSpawn" 0 1e+02 0.0 (Math|Random|RandomFloatinRange 5.0 2e+01) 0.0 1 0))
    (Default|EventTurnAway _returnvalue)))