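; Base vehicle unit Blueprint that moves to targets, auto-attacks them and quakes the ground.
; A looping timer at attack-speed interval rotates it toward an in-range target, then attacks, or resumes movement otherwise.
; The movement query fires a footquake, dealing half damage to nearby other-team actors, when velocity is positive.
; When stuck, it may retarget a nearby living actor via sphere trace; debug prints remain.
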(event Custom|Activate%20Vehicle
  ;[1 1 1] Activate unit (Move To)
  (Components|Sphere|SetSphereRadius (Variables|Default|GetSphere) (Variables|Default|GetAttackRange) true)
  (CallFunction|EventMoveto))

(event Custom|Event_Check%20Distance%20to%20Target
  ;[1 1 1] Check Distance & Rotate To (loop)
  (bind _inrange (CallFunction|CheckDistancetoTarget (Variables|Default|GetAttackRange)))
  (if _inrange
    (CallFunction|EventRotatetoTarget "None" false)
    (else
      (Variables|Default|Set_moving false)
      (CallFunction|EventMoveto))))

(event Custom|Event_AttackObstruction
  (bind _returnvalue (Transformation|GetActorLocation))
  (bind _target (Variables|Default|GetTarget))
  ;[1 1 1] Attack obstructed
  (Development|PrintString "STUCK ON SOMETHING")
  (Variables|Default|Set_moving false)
  (if (not (Variables|Default|Get_rotating))
    (Utilities|IsValid _target
      (:Is%20Valid
        (Utilities|Casting|CastToStructure_Master _target))
      (:Is%20Not%20Valid
        _))
    (bind _outhit (Collision|SphereTraceForObjects _returnvalue _returnvalue (Variables|Default|GetAttackRange) (Utilities|Array|MakeArray "ObjectTypeQuery3") false 0 "ForOneFrame"))
    (if (.bBlockingHit (Collision|BreakHitResult _outhit))
      (bind _asactor_master (Utilities|Casting|CastToActor_Master (.HitActor (Collision|BreakHitResult _outhit))))
      (if (not (Variables|/Game/Blueprints/Actors/Masters/Actor_Master.Actor_Master_C|GetIsDead _asactor_master))
        (CallFunction|AgroTarget _asactor_master))
      (else
        (CallFunction|EventMoveto)))))

(event Custom|Event_Footquake
  (bind _returnvalue (Transformation|GetActorLocation))
  (bind _returnvalue_2 (+ _returnvalue "0, 0,-150.000000"))
  ;[1 1 1] footquake
  (Development|PrintString "FOOTQUAKE" true true "(R=1.000000,G=0.037576,B=0.000000,A=1.000000)" 0.2)
  (bind _outhits (Collision|MultiSphereTraceForObjects _returnvalue_2 _returnvalue_2 (* (Variables|Default|GetAttackRange) 0.5) (Utilities|Array|MakeArray "ObjectTypeQuery3") false 0 "None"))
  (for _array_element _outhits
    (bind _asactor_master (Utilities|Casting|CastToActor_Master (.HitActor (Collision|BreakHitResult _array_element))))
    (if (not (== (Variables|/Game/Blueprints/Actors/Masters/Actor_Master.Actor_Master_C|GetTeam _asactor_master) (Variables|Default|GetTeam)))
      (Default|TakeDamage _asactor_master (* (Variables|Default|GetAttackDamage) 0.5) self))))

(event Custom|Event_IsMovingQuery
  ;[1 0.3199 0.28] Is Moving Query
  (if (or (Variables|Default|Get_moving) (Variables|Default|Get_rotating))
    (if (> (Variables|Default|Get_velocity) 0.0)
      (CallFunction|EventFootquake)
      (else
        (CallFunction|EventAttackObstruction)))))

(event EventBeginPlay
  ;[1 1 1] begin play
  (|CallParentFunction)
  (CallFunction|ActivateVehicle)
  (Utilities|FlowControl|Delay 1.0)
  (Utilities|Time|SetTimerbyEvent (delegate Custom|Event_Check%20Distance%20to%20Target) (Utilities|CalculateAttackSpeed (Variables|Default|GetAttackSpeed)) true))

(event EventEventRotatetoTargetEnd
  (params (UsingMove :type Name :default "None") (FirstMove :type Boolean))
  ;[1 1 1] AutoAttack (Rotate End)
  (CallFunction|EventAutoAttack))

(fn ConstructionScript
  (|CallParentFunction))