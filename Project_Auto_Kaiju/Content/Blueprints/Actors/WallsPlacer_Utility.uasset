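; WallsPlacer_Utility is a utility actor that, at BeginPlay, probes a grid of points over its Box component's area.
; Nested loops derive the grid size from the box extents, stepping 100 units and snapping each point through CalculateGridOffset.
; Each point gets a thin vertical sphere trace against WorldDynamic objects with timed debug drawing.
; The trace results are unused, so no walls are placed here.
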(event EventBeginPlay
  (bind _box (Variables|Default|GetBox))
  (bind _boxextent (Variables|/Script/Engine.BoxComponent|GetBoxExtent _box))
  (for _index (range 1 (Math|Float|Truncate (* (.x _boxextent) 0.015)))
    (for _index_2 (range 1 (Math|Float|Truncate (* (.y _boxextent) 0.015)))
      (Collision|SphereTraceForObjects (+ (Utilities|CalculateGridOffset (+ (+ (Transformation|GetWorldLocation (Variables|Default|GetBox)) (Math|Vector|MakeVector (* (- _index 1) 1e+02) (* (- _index_2 1) 1e+02) 0.0)) (Math|Vector|MakeVector (* (.x _boxextent) -0.5) (* (.y _boxextent) -0.5) 0.0)) "0.000000,0.000000,0") "0, 0,500.000000") (+ (Utilities|CalculateGridOffset (+ (+ (Transformation|GetWorldLocation (Variables|Default|GetBox)) (Math|Vector|MakeVector (* (- _index 1) 1e+02) (* (- _index_2 1) 1e+02) 0.0)) (Math|Vector|MakeVector (* (.x _boxextent) -0.5) (* (.y _boxextent) -0.5) 0.0)) "0.000000,0.000000,0") "0, 0,-1000.000000") 1.0 (Utilities|Array|MakeArray "ObjectTypeQuery2") false 0 "ForDuration"))))

(fn ConstructionScript
  (|CallParentFunction))