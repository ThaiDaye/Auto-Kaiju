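; Player actor for a kaiju auto-battler: handles pre-battle unit placement, starting the simulation and detecting win or loss.
; Mouse sphere traces drive picking up, dragging and dropping Kaiju onto slots or grid-snapped ground; merging only prints.
; SpawnKaiju fills the lowest free bench slot, and StartSimulation activates units outside slots.
; Looping timers count living enemies and Kaiju on board or bench to decide the result, currently shown via PrintString.
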(event Custom|CheckEnemyNumbers
  ;[1 1 1] check game status
  (bind (_enemy _energy_structures _structures) (CallFunction|CheckEnemiesinGame))
  (Variables|Default|Set_enemyOnBoard _enemy)
  (Variables|Default|Set_energyStructuresOnBoard _energy_structures)
  (Variables|Default|Set_structuresOnBoard _structures)
  (CallFunction|CheckGameEndState))

(event Custom|CheckKaijuNumbers
  ;[1 1 1] check game status
  (bind (_onboard _onbench) (CallFunction|CheckKaijuinGame))
  (Variables|Default|Set_kaijuOnBoard _onboard)
  (Variables|Default|Set_kaijuOnBench _onbench))

(event Custom|ReloadLevel
  ;[1 1 1] reload level
  (bind _returnvalue (Game|GetCurrentLevelName true))
  (Game|OpenLevel(byName) (Utilities|String|StringToName _returnvalue)))

(event EventTick
  (params (DeltaSeconds :type Float%20%28single-precision%29))
  (bind _unit_ref (Variables|Default|GetUnit%20Ref))
  ;[1 1 1] Tick - Set Dragged Actor
  (Utilities|IsValid _unit_ref
    (:Is%20Valid
      (bind (_outhit _mouseonscreen _returnvalue) (CallFunction|TraceUnderCursor "None" (Utilities|Array|MakeArray "ObjectTypeQuery13" "ObjectTypeQuery2")))
      (Transformation|SetActorLocation _unit_ref (select (and _mouseonscreen _returnvalue) (+ (.Location (Collision|BreakHitResult _outhit)) "0.000000, 0,300.000000") (Variables|Default|Get_lastDragLocation)) false false)
      (Variables|Default|Set_lastDragLocation (select (and _mouseonscreen _returnvalue) (+ (.Location (Collision|BreakHitResult _outhit)) "0.000000, 0,300.000000") (Variables|Default|Get_lastDragLocation))))
    (:Is%20Not%20Valid
      (Variables|Default|Set_lastDragLocation "0, 0, 0"))))

(event EventBeginPlay
  (bind _returnvalue (Game|GetPlayerController 0))
  ;[1 1 1] begin play
  (CallFunction|Init)
  (Variables|/Script/Engine.PlayerController|SetbShowMouseCursor _returnvalue true)
  (Variables|/Script/Engine.PlayerController|SetCurrentMouseCursor _returnvalue "Default")
  (Utilities|Time|SetTimerbyEvent (delegate Custom|CheckKaijuNumbers) 0.2 true)
  (Utilities|Time|SetTimerbyEvent (delegate Custom|CheckEnemyNumbers) 0.2 true))

(event Input|MouseEvents|LeftMouseButton
  (params (Key :type Key%20Structure :default "None"))
  (bind _unit_ref (Variables|Default|GetUnit%20Ref))
  ;[1 1 1] Left Mouse Click
  (:Pressed
    (if (not (Variables|Default|Get_simulationStarted))
      (Utilities|IsValid (Variables|Default|GetUnit%20Ref)
        (:Is%20Valid
          (bind (_outhit _mouseonscreen _returnvalue) (CallFunction|TraceUnderCursor "None" (Utilities|Array|MakeArray "ObjectTypeQuery12" "ObjectTypeQuery13")))
          (if (and _mouseonscreen _returnvalue)
            (Utilities|Casting|CastToKaiju_Master (Variables|Default|GetUnit%20Ref))
            (Utilities|Casting|CastToKaiju_Master (.HitActor (Collision|BreakHitResult _outhit))
              (:then
                (Development|PrintString "MERGE KAIJU" true true "(R=1.000000,G=0.610496,B=0.000000,A=1.000000)"))
              (:CastFailed
                (Utilities|Casting|CastToStructure_Master (.HitActor (Collision|BreakHitResult _outhit))
                  (:then
                    (Development|PrintString "CANT PLACE THERE" true true "(R=1.000000,G=0.610496,B=0.000000,A=1.000000)"))
                  (:CastFailed
                    (bind _asslot_utility (Utilities|Casting|CastToSlot_Utility (.HitActor (Collision|BreakHitResult _outhit)))
                      (:then
                        (CallFunction|DropKaiju _unit_ref _asslot_utility "0, 0, 0"))
                      (:CastFailed
                        (CallFunction|DropKaiju _unit_ref 0 (Math|Vector|MakeVector (.X (Math|Vector|BreakVector (.Location (Collision|BreakHitResult _outhit)))) (.Y (Math|Vector|BreakVector (.Location (Collision|BreakHitResult _outhit)))) 0.0))))))))))
        (:Is%20Not%20Valid
          (bind _outhit_2 (CallFunction|TraceUnderCursor "None" (Utilities|Array|MakeArray "ObjectTypeQuery12")))
          (bind _asslot_utility_2 (Utilities|Casting|CastToSlot_Utility (.HitActor (Collision|BreakHitResult _outhit_2)))
            (:then
              (Utilities|IsValid (Variables|/Game/Blueprints/Actors/Utility/Slot_Utility.Slot_Utility_C|GetUnit%20Ref _asslot_utility_2)
                (:Is%20Valid
                  (bind _askaiju_master (Utilities|Casting|CastToKaiju_Master (Variables|/Game/Blueprints/Actors/Utility/Slot_Utility.Slot_Utility_C|GetUnit%20Ref _asslot_utility_2)))
                  (CallFunction|PickUpKaiju _askaiju_master _asslot_utility_2)
                  (Development|PrintString "Actor Picked Up" true true "(R=1.000000,G=0.372144,B=0.000000,A=1.000000)" :!label _label))
                (:Is%20Not%20Valid
                  (Development|PrintString "No Actor in Slot" true true "(R=1.000000,G=0.372144,B=0.000000,A=1.000000)"))))
            (:CastFailed
              (bind _askaiju_master_2 (Utilities|Casting|CastToKaiju_Master (.HitActor (Collision|BreakHitResult _outhit_2))))
              (CallFunction|PickUpKaiju _askaiju_master_2 (Variables|/Game/Blueprints/Actors/Masters/Unit_Master.Unit_Master_C|Get_slotParent _askaiju_master_2))
              (goto _label))))))))

(event Input|KeyboardEvents|R
  (params (Key :type Key%20Structure :default "None"))
  ;[1 1 1] reload level
  (:Pressed
    (bind _returnvalue (Game|GetCurrentLevelName true))
    (Game|OpenLevel(byName) (Utilities|String|StringToName _returnvalue))))

(fn ConstructionScript)

(fn PickUpKaiju
  (params (Unit%20Ref :type Actor%20Master%20Object%20Reference) (Parent :type Slot%20Utility%20Object%20Reference))
  (bind _output_get (Variables|Default|SetUnit%20Ref Unit%20Ref))
  (Transformation|SetActorRotation _output_get)
  (bind _asunit_master (Utilities|Casting|CastToUnit_Master _output_get)
    (:then
      (Variables|/Game/Blueprints/Actors/Masters/Actor_Master.Actor_Master_C|Set_active _asunit_master false)
      (bind _askaiju_master (Utilities|Casting|CastToKaiju_Master _asunit_master)
        (:then
          (Variables|/Game/Blueprints/Actors/Masters/Unit_Master.Unit_Master_C|Set_slotParent _askaiju_master 0)
          (Components|Movement|StopMovementImmediately (Variables|/Script/Engine.Character|GetCharacterMovement _askaiju_master))
          (Collision|SetCollisionEnabled (Variables|/Game/Blueprints/Actors/Kaiju_Master.Kaiju_Master_C|GetSlot%20Collision _askaiju_master) "NoCollision"))
        (:CastFailed
          _)))
    (:CastFailed
      _))
  (Utilities|IsValid Parent
    (:Is%20Valid
      (Variables|/Game/Blueprints/Actors/Utility/Slot_Utility.Slot_Utility_C|SetUnit%20Ref Parent 0))))

(fn TraceUnderCursor
  (params (DrawDebugType :type EDrawDebugTrace%20Enum :default "None") (ObjectTypes :type Array%20of%20EObjectTypeQuery%20Enums :default "ObjectTypeQuery1"))
  (bind _returnvalue (Game|GetPlayerController 0))
  (bind _camera (Variables|Default|GetCamera))
  (bind (_worldlocation _worlddirection _returnvalue_2) (Game|Player|ConvertMouseLocationToWorldSpace _returnvalue))
  (bind _returnvalue_3 (Transformation|GetWorldLocation _camera))
  (bind (_outhit _returnvalue_4) (Collision|SphereTraceForObjects _returnvalue_3 (+ _returnvalue_3 (* (Math|Rotator|GetRotationXVector (Math|Rotator|FindLookatRotation _returnvalue_3 _worldlocation)) 1e+04)) 25.0 ObjectTypes false 0 DrawDebugType true "(R=1.000000,G=0.000000,B=0.229848,A=1.000000)" "(R=1.000000,G=0.823764,B=0.000000,A=1.000000)" 0.5))
  (return _outhit _returnvalue_2 _returnvalue_4))

(fn DropKaiju
  (params (Unit :type Actor%20Master%20Object%20Reference) (Drop%20Slot :type Slot%20Utility%20Object%20Reference) (Drop%20Location :type Vector))
  (bind _returnvalue (- Drop%20Location "-100.000000, 0, 0"))
  (bind _grid_location (Utilities|CalculateGridOffset _returnvalue "0,0,100.000000"))
  (Utilities|IsValid Drop%20Slot
    (:Is%20Valid
      (switch Utilities|FlowControl|Switch|SwitchonDragSlot_Type (Variables|/Game/Blueprints/Actors/Utility/Slot_Utility.Slot_Utility_C|GetSlot%20Type Drop%20Slot)
        (:NewEnumerator1
          _)
        (:NewEnumerator3
          _))
      (if (Utilities|Enum|Equal(Enum) (Variables|/Game/Blueprints/Actors/Masters/Actor_Master.Actor_Master_C|GetUnit%20Type Unit) "NewEnumerator0")
        (Utilities|IsValid (Variables|Default|GetUnit%20Ref)
          (:Is%20Valid
            (Transformation|SetActorLocation (Variables|Default|GetUnit%20Ref) (Transformation|GetActorLocation Drop%20Slot) false false))
          (:Is%20Not%20Valid
            _))
        (bind _asunit_master (Utilities|Casting|CastToUnit_Master Unit)
          (:then
            (Variables|/Game/Blueprints/Actors/Masters/Unit_Master.Unit_Master_C|Set_slotParent _asunit_master Drop%20Slot))
          (:CastFailed
            _))
        (Variables|/Game/Blueprints/Actors/Utility/Slot_Utility.Slot_Utility_C|SetUnit%20Ref Drop%20Slot Unit)
        (bind _askaiju_master (Utilities|Casting|CastToKaiju_Master Unit :!label _label))
        (Collision|SetCollisionEnabled (Variables|/Game/Blueprints/Actors/Kaiju_Master.Kaiju_Master_C|GetSlot%20Collision _askaiju_master) "QueryAndPhysics")
        (Variables|/Game/Blueprints/Actors/Masters/Unit_Master.Unit_Master_C|Set_slotParent _askaiju_master Drop%20Slot)
        (Variables|Default|SetUnit%20Ref 0)
        (Variables|Default|Set_lastDragLocation "0, 0, 0")))
    (:Is%20Not%20Valid
      (bind _returnvalue_2 (Collision|SphereTraceForObjects _grid_location _grid_location 25.0 (Utilities|Array|MakeArray "ObjectTypeQuery3") false 0 "None"))
      (if _returnvalue_2
        (Development|PrintString "CANT PLACE THERE" true true "(R=1.000000,G=0.610496,B=0.000000,A=1.000000)")
        (else
          (Transformation|SetActorLocation (Variables|Default|GetUnit%20Ref) _grid_location false false)
          (goto _label))))))

(fn StartSimulation
  (Variables|Default|Set_simulationStarted true)
  (bind _outactors (Actor|GetAllActorsOfClass "/Game/Blueprints/Actors/Masters/Actor_Master.Actor_Master_C"))
  (for _array_element _outactors
    (bind _asunit_master (Utilities|Casting|CastToUnit_Master _array_element)
      (:then
        (Utilities|IsValid (Variables|/Game/Blueprints/Actors/Masters/Unit_Master.Unit_Master_C|Get_slotParent _asunit_master)
          (:Is%20Valid
            (Variables|/Game/Blueprints/Actors/Masters/Actor_Master.Actor_Master_C|Set_active _array_element false))
          (:Is%20Not%20Valid
            (Variables|/Game/Blueprints/Actors/Masters/Actor_Master.Actor_Master_C|Set_active _array_element true :!label _label)
            (bind _asvehicle_master (Utilities|Casting|CastToVehicle_Master _asunit_master)
              (:then
                (Default|ActivateVehicle _asvehicle_master))
              (:CastFailed
                (bind _askaiju_master (Utilities|Casting|CastToKaiju_Master _asunit_master))
                (Default|ActivateKaiju _askaiju_master))))))
      (:CastFailed
        (goto _label)))))

(fn SumulationFinished
  (params (Win :type Boolean))
  (if (not (Variables|Default|Get_simulationFinished))
    (Variables|Default|Set_simulationFinished true)
    (if Win
      (Development|PrintString "YOU WIN" true true "(R=0.000000,G=1.000000,B=0.266184,A=1.000000)" 1e+01)
      (else
        (Development|PrintString "YOU LOSE" true true "(R=1.000000,G=0.000000,B=0.000000,A=1.000000)" 1e+01)))))

(fn Init
  (bind _outactors (Actor|GetAllActorsOfClass "/Game/Blueprints/Actors/Masters/Actor_Master.Actor_Master_C"))
  (for _array_element _outactors
    (Variables|/Game/Blueprints/Actors/Masters/Actor_Master.Actor_Master_C|Set_active _array_element false)
    (Components|Movement|StopMovementImmediately (Variables|/Script/Engine.Character|GetCharacterMovement _array_element))))

(fn CheckKaijuinGame
  (bind _outactors (Actor|GetAllActorsOfClass "/Game/Blueprints/Actors/Kaiju_Master.Kaiju_Master_C"))
  (for _array_element _outactors
    (Utilities|IsValid (Variables|/Game/Blueprints/Actors/Masters/Unit_Master.Unit_Master_C|Get_slotParent _array_element)
      (:Is%20Valid
        (LocalVariables|Setbench (+ (LocalVariables|Getbench) 1)))
      (:Is%20Not%20Valid
        (LocalVariables|Setboard (+ (LocalVariables|Getboard) 1)))))
  (return (LocalVariables|Getboard) (LocalVariables|Getbench)))

(fn CheckEnemiesinGame
  (bind _outactors (Actor|GetAllActorsOfClass "/Game/Blueprints/Actors/Masters/Actor_Master.Actor_Master_C"))
  (for _array_element _outactors
    (bind _asvehicle_master (Utilities|Casting|CastToVehicle_Master _array_element)
      (:then
        (if (not (Variables|/Game/Blueprints/Actors/Masters/Actor_Master.Actor_Master_C|GetIsDead _asvehicle_master))
          (LocalVariables|SetEnemyBoard (+ (LocalVariables|GetEnemyBoard) 1))))
      (:CastFailed
        (bind _asstructure_master (Utilities|Casting|CastToStructure_Master _array_element))
        (if (not (Variables|/Game/Blueprints/Actors/Masters/Actor_Master.Actor_Master_C|GetIsDead _asstructure_master))
          (switch Utilities|FlowControl|Switch|SwitchonUnit_Type (Variables|/Game/Blueprints/Actors/Masters/Actor_Master.Actor_Master_C|GetUnit%20Type _asstructure_master)
            (:NewEnumerator1
              (LocalVariables|SetStructure (+ (LocalVariables|GetStructure) 1) :!label _label))
            (:NewEnumerator3
              (LocalVariables|SetEnergyStructure (+ (LocalVariables|GetEnergyStructure) 1)))
            (:NewEnumerator6
              (goto _label)))))))
  (return (LocalVariables|GetEnemyBoard) (LocalVariables|GetEnergyStructure) (LocalVariables|GetStructure)))

(fn CheckGameEndState
  (if (Math|Boolean|ANDBoolean (Variables|Default|Get_simulationStarted) (== (Variables|Default|Get_enemyOnBoard) 0) (== (Variables|Default|Get_energyStructuresOnBoard) 0))
    (CallFunction|SumulationFinished true)
    (elif (and (Variables|Default|Get_simulationStarted) (== (Variables|Default|Get_kaijuOnBoard) 0))
      (CallFunction|SumulationFinished false))))

(fn SpawnKaiju
  (bind _outactors (Actor|GetAllActorsOfClass "/Game/Blueprints/Actors/Utility/Slot_Utility.Slot_Utility_C"))
  (bind _output_get (LocalVariables|SetNewLocalVar_0 _outactors))
  (for (_array_element _array_index) _output_get
    (if (Utilities|Enum|Equal(Enum) (Variables|/Game/Blueprints/Actors/Utility/Slot_Utility.Slot_Utility_C|GetSlot%20Type _array_element) "NewEnumerator1")
      (Utilities|IsValid (Variables|/Game/Blueprints/Actors/Utility/Slot_Utility.Slot_Utility_C|GetUnit%20Ref _array_element)
        (:Is%20Not%20Valid
          (if (<= (Variables|/Game/Blueprints/Actors/Utility/Slot_Utility.Slot_Utility_C|GetSlot%20Number _array_element) (LocalVariables|GetSmallestNum))
            (LocalVariables|SetSmallestNum (Variables|/Game/Blueprints/Actors/Utility/Slot_Utility.Slot_Utility_C|GetSlot%20Number _array_element))
            (LocalVariables|SetSmallestNumID _array_index)
            (LocalVariables|SetFound true))))))
  (if (LocalVariables|GetFound)
    (Development|PrintString "UNIT BOUGHT!" true true "(R=0.021003,G=0.000000,B=1.000000,A=1.000000)")
    (bind _returnvalue (AI|SpawnAIFromClass "/Game/Blueprints/Actors/Kaiju_Master.Kaiju_Master_C" 0 (+ (Transformation|GetActorLocation (Utilities|Array|Get(acopy) _output_get (LocalVariables|GetSmallestNumID))) "0, 0,150.000000") "0, 0, 0" false 0))
    (bind _askaiju_master (Utilities|Casting|CastToKaiju_Master _returnvalue))
    (CallFunction|DropKaiju _askaiju_master (Utilities|Array|Get(acopy) _output_get (LocalVariables|GetSmallestNumID)) "0, 0, 0")
    (else
      (Development|PrintString "NO ROOM FOR UNIT!" true true "(R=0.021003,G=0.000000,B=1.000000,A=1.000000)"))))