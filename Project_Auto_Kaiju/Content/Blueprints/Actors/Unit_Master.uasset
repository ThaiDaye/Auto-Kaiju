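; Unit_Master is a base Blueprint for mobile units, extending a parent class with movement setup and target selection.
; Initiate Unit runs the parent logic, derives walk speed from MoveSpeed and zeroes Power.
; Get Target handles Kaiju units by scanning all Structure_Master actors for the closest EnergyStructure under the stored Distance, falling back to BlockStructure if none qualifies.
; Distance is not reset within the search.
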(event EventBeginPlay
  (|CallParentFunction))

(fn ConstructionScript
  (|CallParentFunction))

(fn InitiateUnit
  (|CallParentFunction)
  (Variables|/Script/Engine.CharacterMovementComponent|SetMaxWalkSpeed (Variables|Character|GetCharacterMovement) (Utilities|CalculateMovespeed (Variables|Default|GetMoveSpeed)))
  (Variables|Default|SetPower 0.0))

(fn GetTarget
  (switch Utilities|FlowControl|Switch|SwitchonUnit_Type (Variables|Default|GetUnit%20Type)
    (:NewEnumerator0
      (Variables|Default|SetTarget 0)
      (bind _outactors (Actor|GetAllActorsOfClass "/Game/Blueprints/Actors/Structure_Master.Structure_Master_C"))
      (for _array_element _outactors
        (if (Utilities|Enum|Equal(Enum) (Variables|/Game/Blueprints/Actors/Actor_Master.Actor_Master_C|GetUnit%20Type _array_element) "NewEnumerator3")
          (if (< (Transformation|GetDistanceTo _array_element) (LocalVariables|GetDistance))
            (LocalVariables|SetDistance (Transformation|GetDistanceTo _array_element))
            (Variables|Default|SetTarget _array_element))))
      (Utilities|IsValid (Variables|Default|GetTarget)
        (:Is%20Not%20Valid
          (for _array_element_2 _outactors
            (if (Utilities|Enum|Equal(Enum) (Variables|/Game/Blueprints/Actors/Actor_Master.Actor_Master_C|GetUnit%20Type _array_element_2) "NewEnumerator1")
              (if (< (Transformation|GetDistanceTo _array_element_2) (LocalVariables|GetDistance))
                (LocalVariables|SetDistance (Transformation|GetDistanceTo _array_element_2))
                (Variables|Default|SetTarget _array_element_2)))))))))