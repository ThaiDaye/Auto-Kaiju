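; General_FunctionLibrary provides FindStatRank, which converts a named stat's value into a numeric rank and letter grade.
; It reads that stat's thresholds from StatRanking_Table and tests them from highest to lowest, returning the first grade reached.
; S+ and S both test StatMaxS, so S is unreachable.
; A missing row or a value below the E threshold returns rank 0, "F", making the StatMaxF check redundant.
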(fn FindStatRank
  (params (StatName :type Name) (Value :type Float%20%28single-precision%29))
  (bind _returnvalue (Utilities|GetDataTableRow "/Game/Blueprints/Data/StatRanking_Table.StatRanking_Table" StatName)
    (:then
      (if (>= Value (.StatMaxS+ (Utilities|Struct|BreakStatRanking_Struct _returnvalue)))
        (return 7 "S+")
        (elif (>= Value (.StatMaxS (Utilities|Struct|BreakStatRanking_Struct _returnvalue)))
          (return 6 "S")
          (elif (>= Value (.StatMaxA (Utilities|Struct|BreakStatRanking_Struct _returnvalue)))
            (return 5 "A")
            (elif (>= Value (.StatMaxB (Utilities|Struct|BreakStatRanking_Struct _returnvalue)))
              (return 4 "B")
              (elif (>= Value (.StatMaxC (Utilities|Struct|BreakStatRanking_Struct _returnvalue)))
                (return 3 "C")
                (elif (>= Value (.StatMaxD (Utilities|Struct|BreakStatRanking_Struct _returnvalue)))
                  (return 2 "D")
                  (elif (>= Value (.StatMaxE (Utilities|Struct|BreakStatRanking_Struct _returnvalue)))
                    (return 1 "E")
                    (elif (>= Value (.StatMaxF (Utilities|Struct|BreakStatRanking_Struct _returnvalue)))
                      _
                      (else
                        _))))))))))
    (:RowNotFound
      _))
  (return 0 "F"))